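; MovingPlateforms is an actor Blueprint for a platform that moves on its own, driven by the Moving timeline.
; At BeginPlay the timeline jumps to a random start time, so separate instances can move out of step.
; Each update sets the Platform's relative location from the Movement vector track, scaling Y, without sweep, and calls Play on the timeline.
; The construction script is empty, and some unused movement nodes remain in the graph.
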(event `self.ReceiveBeginPlay`
  (bind (_direction _movement) (`Timeline|Moving` :`NewTime` (* (`KismetMathLibrary.RandomFloat`) 10.0) :!via `SetNewTime` :!label _label)
    (:`Update`
      (bind (_x _y _z) (`KismetMathLibrary.BreakVector3f` _movement))
      (`SceneComponent.K2_SetRelativeLocation` (`self.platform`) (`KismetMathLibrary.MakeVector` _x (* _y 205.0) _z) false false)
      (goto _label))))

(fn `UserConstructionScript`)